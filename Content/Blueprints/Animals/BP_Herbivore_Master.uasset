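; Master herbivore Blueprint that sends the animal toward a resource suited to the time of day.
; On BeginPlay it copies the game mode's resource map, starts a move, then binds to GM_GameMode's dawn, dusk and night events.
; Each event changes the needed resource type and moves again via AI MoveTo.
; Despite its name, FindClosestResource targets a reachable point near a randomly chosen matching resource, ignoring distance.
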(event `self.ReceiveBeginPlay`
  (bind _resourcemap (message `/Game/Blueprints/Interfaces/BPI_ResourceType.GetResources` (`GameplayStatics.GetGameMode`)))
  (set `self.Resource Map` _resourcemap)
  (`self.FindClosestResource`)
  (bind _asgm_game_mode (cast `/Game/Blueprints/Core/GM_GameMode` (`GameplayStatics.GetGameMode`)))
  (bind _output_get (set `self.As GM Game Mode` _asgm_game_mode))
  (add `/Game/Blueprints/Core/GM_GameMode.SetDawn` _output_get (delegate `SetDawn`))
  (add `/Game/Blueprints/Core/GM_GameMode.SetDusk` (`self.As GM Game Mode`) (delegate `SetDusk`))
  (add `/Game/Blueprints/Core/GM_GameMode.SetNight` (`self.As GM Game Mode`) (delegate `SetNight`)))

(event `SetDawn`
  (set `self.ResourceNeeded` "NewEnumerator1")
  (`self.FindClosestResource`))

(event `SetDusk`
  (set `self.ResourceNeeded` "NewEnumerator2")
  (`self.FindClosestResource`))

(event `SetNight`
  (set `self.ResourceNeeded` "NewEnumerator0")
  (`self.FindClosestResource`))

(event `FindClosestResource`
  (bind _closestresource (`self.SearchForResource`))
  (`AITask_MoveTo.AIMoveTo` (`AIBlueprintHelperLibrary.GetAIController` self) (`NavigationSystemV1.K2_GetRandomReachablePointInRadius` _closestresource 400.0 null null) null))

(fn `SearchForResource`
  (returns (ClosestResource :type "Vector Structure"))
  (locals (SearchPoint :type "Vector Structure") (isFirstPosition :type Boolean) (ArrayIndex :type Integer) (ResourceActors :type "Array of Actor Object Reference") (ClosestPoints :type "Array of Vector Structure") (SearchResourceActor :type "Actor Object Reference"))
  (bind _resourceactors (`local.ResourceActors`))
  (bind _values (`BlueprintMapLibrary.Map_Values` (`self.Resource Map`)))
  (for (_array_element _array_index) _values
    (set `local.ArrayIndex` _array_index)
    (if (== _array_element (`self.ResourceNeeded`))
      (bind _keys (`BlueprintMapLibrary.Map_Keys` (`self.Resource Map`)))
      (`KismetArrayLibrary.Array_Add` (`local.ResourceActors`) (`|GetArrayItem` _keys (`local.ArrayIndex`)))))
  (return (`self.K2_GetActorLocation` (`|GetArrayItem` _resourceactors (`KismetMathLibrary.RandomInteger` (`KismetArrayLibrary.Array_Length` _resourceactors))))))

(fn `UserConstructionScript`)