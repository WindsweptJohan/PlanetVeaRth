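; BP_MasterResource is a resource actor that carries a resource type and shows its name on a text component set in the construction script.
; On BeginPlay it reports itself and its type to the game mode.
; GetResourcePosition returns a random LocationArray offset added to the actor's location.
; GetResourceActor and GetResources are empty, and a TESTReference event swaps the mesh material to CubeMaterial.
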(event `self.ReceiveBeginPlay`
  (message `/Game/Blueprints/Interfaces/BPI_ResourceType.SetSendResource` (`GameplayStatics.GetGameMode`) self (`self.ResoureceType`)))

(event `/Game/Blueprints/Interfaces/BPI_ResourceType.TESTReference`
  (`PrimitiveComponent.SetMaterial` (`self.StaticMesh`) 0 "/Game/Assets/Meshes/CubeMaterial.CubeMaterial"))

(fn `GetResourceActor`
  (returns (FoodRef :type "Actor Object Reference") (WaterRef :type "Actor Object Reference") (SleepRef :type "Actor Object Reference"))
  (return null null null))

(fn `GetResourcePosition`
  (returns (NewParam :type "Vector Structure"))
  (bind _locationarray (`self.LocationArray`))
  (return (+ (`|GetArrayItem` _locationarray (`KismetMathLibrary.RandomIntegerInRange` 0 (`KismetArrayLibrary.Array_LastIndex` _locationarray))) (`self.K2_GetActorLocation`))))

(fn `GetResources`
  (returns (ResourceMap :type "Map of Actor Object Reference to /Game/Blueprints/Enums/En_ResourceType Enum"))
  (return))

(fn `UserConstructionScript`
  (`TextRenderComponent.K2_SetText` (`self.ResourceType`) (`KismetTextLibrary.Conv_StringToText` (`|GetEnumeratorNameAsString` (`self.ResoureceType`)))))