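; Base character Blueprint for herbivore animals that sleep, drink and eat to meet resource needs.
; On BeginPlay it applies a random uniform mesh scale for variation, and an event sets walk speed.
; SetatLocation asks the AI controller which resource is needed and calls the matching sleep, drink or eat action.
; Its own resource getters are stubs returning empty or fixed defaults.
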(event `/Game/Blueprints/Interfaces/BPI_AIToAnimal.SetWalkSpeed`
  (params (NewSpeed :type "Float (single-precision)"))
  (set `CharacterMovementComponent.MaxWalkSpeed` NewSpeed (`self.CharacterMovement`)))

(event `self.ReceiveBeginPlay`
  (set `self.RandomScale` (`KismetMathLibrary.RandomFloatInRange` (`self.MinScale`) (`self.MaxScale`)))
  (`SceneComponent.SetWorldScale3D` (`self.Mesh`) (`KismetMathLibrary.MakeVector` (`self.RandomScale`) (`self.RandomScale`) (`self.RandomScale`))) ; Sets random scale on beingplay for variation
)

(event `/Game/Blueprints/Interfaces/BPI_AIToAnimation.SetAtLocation`
  (params (Resource :type "/Game/Blueprints/Enums/En_ResourceType Enum" :default "NewEnumerator0"))
  (bind _resource (message `/Game/Blueprints/Interfaces/BPI_AIToAnimal.GetResourceNeeded` (`AIBlueprintHelperLibrary.GetAIController` self)))
  (switch `/Game/Blueprints/Enums/En_ResourceType` _resource
    (:`NewEnumerator0`
      (`self.Sleep`))
    (:`NewEnumerator1`
      (`self.Drink`))
    (:`NewEnumerator2`
      (`self.Eat`))))

(fn `GetResourceActor`
  (returns (FoodRef :type "Actor Object Reference") (WaterRef :type "Actor Object Reference") (SleepRef :type "Actor Object Reference"))
  (return null null null))

(fn `GetResourceNeeded`
  (returns (Resource :type "/Game/Blueprints/Enums/En_ResourceType Enum"))
  (return "NewEnumerator0"))

(fn `GetResourcePosition`
  (returns (NewParam :type "Vector Structure"))
  (return (0.0 0.0 0.0)))

(fn `UserConstructionScript`)