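; Handheld camera actor that motion controllers pick up and drop, letting the player take photos and browse them on its display.
; Photos are copied from the SceneCapture2D render target into a Texture2D array, with a temporary gamma boost and optional timeline-driven spotlight flash.
; A dynamic material switches the display between widget render target, capture feed and saved photos.
; Shutter and brightness button events scroll the gallery while it is open.
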(event `self.ReceiveBeginPlay`
  (bind _display (`self.Display`))
  (`self.EnableInput` (`GameplayStatics.GetPlayerController` 0))
  ;[1 1 1] Intercept Render Target for display
  (`KismetSystemLibrary.Delay` 0.6)
  (bind _returnvalue (`PrimitiveComponent.CreateDynamicMaterialInstance` _display 0 (`PrimitiveComponent.GetMaterial` _display 0) "None"))
  (`MaterialInstanceDynamic.SetTextureParameterValue` _returnvalue "RenderTexture" (`WidgetComponent.GetRenderTarget` (`self.Widget`)))
  (`PrimitiveComponent.SetMaterial` (`self.Display`) 0 _returnvalue))

(event `/Game/VirtualRealityBP/Blueprints/PickupActorInterface.Pickup`
  (params (AttachTo :type "SceneComponent Object Reference"))
  ;[1 1 1] Player picks up / Drops camera
  (`PrimitiveComponent.SetSimulatePhysics` (`self.StaticMeshComponent`) false)
  (`SceneComponent.K2_AttachToComponent` (`self.K2_GetRootComponent`) AttachTo "None" "KeepWorld" "KeepWorld" "KeepWorld" true))

(event `/Game/VirtualRealityBP/Blueprints/PickupActorInterface.Drop`
  ;[1 1 1] Player picks up / Drops camera
  (`PrimitiveComponent.SetSimulatePhysics` (`self.StaticMeshComponent`) true)
  (`self.K2_DetachFromActor` "KeepWorld" "KeepWorld" "KeepWorld"))

(event `/Game/Blueprints/Interfaces/BPI_PhotoCamera.SetTakePhoto`
  (bind _savedphototexturearray (`self.SavedPhotoTextureArray`))
  ;[0 0.1696 1] Player takes photo
  (set `self.isInGallery` false)
  (if (`self.isFlash`)
    (`self.CameraFlash`)
    (`KismetSystemLibrary.Delay` 0.05))
  (set `TextureRenderTarget.TargetGamma` 1.75 (`SceneCaptureComponent2D.TextureTarget` (`self.SceneCaptureComponent2D`))) ; Set gamma to avoid darker pictures
  (`KismetSystemLibrary.Delay` 0.0) ; Skip one frame
  (`KismetSystemLibrary.Delay` 0.0)
  (`self.SavePictureToArray`)
  (set `TextureRenderTarget.TargetGamma` 0.0 (`SceneCaptureComponent2D.TextureTarget` (`self.SceneCaptureComponent2D`)))
  (`self.SetGalleryScrollBool` false true)
  (`MaterialInstanceDynamic.SetTextureParameterValue` (`self.DMI_Display`) "RenderTexture" (`|GetArrayItem` _savedphototexturearray (`KismetArrayLibrary.Array_LastIndex` _savedphototexturearray)))
  (`KismetSystemLibrary.Delay` 2.0)
  (`MaterialInstanceDynamic.SetTextureParameterValue` (`self.DMI_Display`) "RenderTexture" (`SceneCaptureComponent2D.TextureTarget` (`self.SceneCaptureComponent2D`))))

(event `CameraFlash`
  ;[1 1 1] Camera Flash
  (bind (_direction _alpha) (`Timeline|FlashTimeline` :!via `PlayFromStart`)
    (:`Update`
      (`LightComponent.SetIntensity` (`self.SpotLight`) (`KismetMathLibrary.Lerp` 0.0 17000.0 _alpha)))))

(event `GalleryScrollUp`
  ;[0 0.8188 1] Player view pictures in gallery
  (set `self.currentPhotoDisplayIndex` (`self.ScrollUpInGallery`))
  (`MaterialInstanceDynamic.SetTextureParameterValue` (`self.DMI_Display`) "RenderTexture" (`|GetArrayItem` (`self.SavedPhotoTextureArray`) (`self.currentPhotoDisplayIndex`)))
  (`self.SetGalleryScrollBool` true))

(event `GalleryScrollDown`
  ;[0 0.8188 1] Player view pictures in gallery
  (set `self.currentPhotoDisplayIndex` (`self.ScrollDownInGallery`))
  (`MaterialInstanceDynamic.SetTextureParameterValue` (`self.DMI_Display`) "RenderTexture" (`|GetArrayItem` (`self.SavedPhotoTextureArray`) (`self.currentPhotoDisplayIndex`)))
  (`self.SetGalleryScrollBool` false))

(event `/Game/Blueprints/Interfaces/BPI_PhotoCamera.SetDisplayGallery`
  (bind _savedphototexturearray (`self.SavedPhotoTextureArray`))
  ;[1 1 1] Recieves input from interactable widget
  (if (not (`self.isInGallery`))
    (set `self.isInGallery` true)
    (`MaterialInstanceDynamic.SetTextureParameterValue` (`self.DMI_Display`) "RenderTexture" (`|GetArrayItem` _savedphototexturearray (`KismetArrayLibrary.Array_LastIndex` _savedphototexturearray)))
    (else
      (set `self.isInGallery` false))))

(event `/Game/Blueprints/Interfaces/BPI_UI.SetShutterButtonPressed`
  ;[1 1 1] Recieves input from interactable widget
  (if (`self.isInGallery`)
    (`self.GalleryScrollDown`)
    (`KismetSystemLibrary.PrintString` "                                                                                                                                              Scroll down")))

(event `/Game/Blueprints/Interfaces/BPI_UI.SetBrightnessButtonPressed`
  ;[1 1 1] Recieves input from interactable widget
  (if (`self.isInGallery`)
    (`self.GalleryScrollUp`)
    (`KismetSystemLibrary.PrintString` "                                                                                                                                              Scroll up")))

(event `/Game/Blueprints/Interfaces/BPI_UI.SetFlashButtonPressed`
  ;[1 1 1] Recieves input from interactable widget
  (bind _isa (`/Engine/EditorBlueprintResources/StandardMacros.FlipFlop`)
    (:`A`
      _)
    (:`B`
      _))
  (bind _output_get (set `self.isFlash` _isa))
  (`KismetSystemLibrary.PrintString` (`KismetStringLibrary.Concat_StrStr` "                                                                                                                                        Flash set to: " (`KismetStringLibrary.Conv_BoolToString` _output_get))))

(fn `GetRenderTexture`
  (returns (`2D Texture Renderer` :type "TextureRenderTarget2D Object Reference"))
  (return null))

(fn `SavePictureToArray`
  (bind (_width _height _pixels) (`LowEntryExtendedStandardLibrary.TextureRenderTarget2DToPixels` (`SceneCaptureComponent2D.TextureTarget` (`self.SceneCaptureComponent2D`))))
  (bind _returnvalue (`LowEntryExtendedStandardLibrary.PixelsToTexture2D` _width _height _pixels))
  (bind _returnvalue_2 (`KismetArrayLibrary.Array_Add` (`self.SavedPhotoTextureArray`) _returnvalue))
  (set `self.currentPhotoDisplayIndex` _returnvalue_2))

(fn `ScrollDownInGallery`
  (returns (ReturnValue :type Integer))
  (return (`KismetMathLibrary.SelectInt` (`KismetMathLibrary.SelectInt` (- (`self.currentPhotoDisplayIndex`) 1) (`KismetMathLibrary.SelectInt` (- (`self.currentPhotoDisplayIndex`) 1) (`KismetArrayLibrary.Array_LastIndex` (`self.SavedPhotoTextureArray`)) (`self.isScrollUp`)) (`self.isScrollDown`)) (`KismetArrayLibrary.Array_LastIndex` (`self.SavedPhotoTextureArray`)) (!= 0 (`self.currentPhotoDisplayIndex`)))))

(fn `ScrollUpInGallery`
  (returns (ReturnValue :type Integer))
  (bind _returnvalue (`KismetArrayLibrary.Array_LastIndex` (`self.SavedPhotoTextureArray`)))
  (return (`KismetMathLibrary.SelectInt` (`KismetMathLibrary.SelectInt` (+ (`self.currentPhotoDisplayIndex`) 1) (`KismetMathLibrary.SelectInt` (+ (`self.currentPhotoDisplayIndex`) 1) (`KismetArrayLibrary.Array_LastIndex` (`self.SavedPhotoTextureArray`)) (`self.isScrollDown`)) (`self.isScrollUp`)) (select `bool` (`KismetMathLibrary.BooleanNOR` (`self.isScrollDown`) (`self.isScrollUp`)) :`true` _returnvalue) (!= _returnvalue (`self.currentPhotoDisplayIndex`)))))

(fn `SetGalleryScrollBool`
  (params (isScrollUp :type Boolean) (ResetBoth :type Boolean))
  (if ResetBoth
    (set `self.isScrollUp` false)
    (set `self.isScrollDown` false)
    (else
      (set `self.isScrollUp` isScrollUp)
      (set `self.isScrollDown` (not isScrollUp)))))

(fn `UserConstructionScript`
  (bind _returnvalue (`KismetMaterialLibrary.CreateDynamicMaterialInstance` "/Game/Assets/Camera/M_Inst_ScreenCapture.M_Inst_ScreenCapture"))
  (bind _output_get (set `self.DMI_Display` _returnvalue))
  (`PrimitiveComponent.SetMaterial` (`self.Display`) 0 _output_get))