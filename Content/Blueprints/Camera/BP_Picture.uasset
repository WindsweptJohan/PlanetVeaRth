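; Camera picture actor that takes a snapshot of the scene through a SceneCaptureComponent2D.
; On BeginPlay it captures the scene once, then passes itself to the Game Mode through a SetSendRenderReference message.
; GetRenderTexture exposes the capture component's texture target, while its own SetSendRenderReference implementation is empty.
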(event `self.ReceiveBeginPlay`
  (`SceneCaptureComponent2D.CaptureScene` (`self.SceneCaptureComponent2D`))
  (message `/Game/Blueprints/Interfaces/BPI_PhotoCamera.SetSendRenderReference` (`GameplayStatics.GetGameMode`) self))

(fn `GetRenderTexture`
  (returns (`2D Texture Renderer` :type "TextureRenderTarget2D Object Reference"))
  (return (`SceneCaptureComponent2D.TextureTarget` (`self.SceneCaptureComponent2D`))))

(fn `SetSendRenderReference`
  (params (Ref :type "Actor Object Reference"))
  (return))

(fn `UserConstructionScript`)