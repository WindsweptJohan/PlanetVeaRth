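; Game mode Blueprint that acts as a shared store for time of day, resource actors and saved photo render references.
; Setter events store the time of day, map each actor to a resource type, and add render references indexed by an incrementing saved photo count.
; Getters return the time of day and the resource map, while GetRenderTexture returns no value.
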(event `/Game/Blueprints/Interfaces/BPI_TimeOfDay.SetSendTimeOfDay`
  (params (TimeOfDay :type Integer))
  (set `self.Time Of Day` TimeOfDay))

(event `/Game/Blueprints/Interfaces/BPI_ResourceType.SetSendResource`
  (params (Actor :type "Actor Object Reference") (Type :type "/Game/Blueprints/Enums/En_ResourceType Enum" :default "NewEnumerator0"))
  (`BlueprintMapLibrary.Map_Add` (`self.ResourceMap`) Actor Type))

(event `/Game/Blueprints/Interfaces/BPI_PhotoCamera.SetSendRenderReference`
  (params (Ref :type "Actor Object Reference"))
  (bind _savedphotoamount (`self.savedPhotoAmount`))
  (`BlueprintMapLibrary.Map_Add` (`self.Ref`) _savedphotoamount Ref)
  (`/Engine/EditorBlueprintResources/StandardMacros.IncrementInt` _savedphotoamount))

(fn `GetRenderTexture`
  (returns (`2D Texture Renderer` :type "TextureRenderTarget2D Object Reference"))
  (return null))

(fn `GetResources`
  (returns (ResourceMap :type "Map of Actor Object Reference to /Game/Blueprints/Enums/En_ResourceType Enum"))
  (return (`self.ResourceMap`)))

(fn `GetTimeOfDay`
  (returns (TimeOfDay :type Integer))
  (return (`self.Time Of Day`)))

(fn `UserConstructionScript`)